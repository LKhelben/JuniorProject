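; Golem enemy AI that starts asleep, wakes when the player enters AwakeCollision, then chases on sight until a timed return to roaming.
; Blackboard flags carry sleep, sighting, roaming and attack state to the AI.
; AttackPlayer picks by distance: a close jump attack spawning an AOE, or a thrown rock projectile, each DoOnce-gated with delayed resets.
; Dark projectile hits subtract the player's Damage from Health and trigger chasing.
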(event `self.ReceiveBeginPlay`
  (`parent.ReceiveBeginPlay`)
  (`BlackboardComponent.SetValueAsBool` (`self.BlackboardRef`) "isAsleep" true))

(event `self.ReceiveTick`
  (params (DeltaSeconds :type "Float (single-precision)"))
  (`|ExecutionSequence`
    (:`then_0`
      (`parent.ReceiveTick` DeltaSeconds))))

(event `self.Attack Player`
  (bind _returnvalue (`self.GetControlRotation`))
  (bind (_returnvalue_roll _returnvalue_pitch _returnvalue_yaw) (`KismetMathLibrary.BreakRotator` (`KismetMathLibrary.RInterpTo` (`self.K2_GetActorRotation`) (`KismetMathLibrary.FindLookAtRotation` (`self.K2_GetActorLocation`) (`self.K2_GetActorLocation` (`GameplayStatics.GetPlayerCharacter` 0))) (`GameplayStatics.GetWorldDeltaSeconds`) 50.0)))
  (if (not (`self.isDead`))
    (set `self.isChasingPlayer` false)
    (bind _asbp_third_person_character_new_base (cast `/Game/ThirdPerson/Blueprints/BP_ThirdPersonCharacter_NewBase` (`GameplayStatics.GetPlayerCharacter` 0)))
    (set `self.CharacterRef` _asbp_third_person_character_new_base)
    (if (not (`self.isAttacking`))
      (if (<= (`self.GetDistanceTo` _asbp_third_person_character_new_base) 500.0)
        (set `self.isAttacking` true)
        (set `self.jumpAttack` true)
        (`/Engine/EditorBlueprintResources/StandardMacros.DoOnce` false :!label _label
          (:`Completed`
            (set `self.Max Walk Speed` 0.0)
            (`KismetSystemLibrary.Delay` 1.75)
            (`|SpawnActorFromClass` "/Game/Characters/AI/AI_golem/BP_AOE.BP_AOE_C" (`SceneComponent.K2_GetComponentToWorld` (`self.Mesh`)) "Undefined" "OverrideRootScale" null null)
            (set `self.jumpAttack` false)
            (`KismetSystemLibrary.PrintString` "Golem is attacking")
            (`KismetSystemLibrary.Delay` 1.6)
            (set `self.Max Walk Speed` 200.0)
            (`BlackboardComponent.SetValueAsBool` (`self.BlackboardRef`) "isAttacking" false)
            (set `self.isChasingPlayer` true)
            (set `self.isAttacking` false)
            (goto _label :!via `Reset`)))
        (else
          (set `self.isAttacking` true)
          (`KismetSystemLibrary.PrintString` "thorwing")
          (`/Engine/EditorBlueprintResources/StandardMacros.DoOnce` false :!label _label_2
            (:`Completed`
              (`self.K2_SetActorRotation` (`KismetMathLibrary.MakeRotator` 0.0 0.0 _returnvalue_yaw))
              (`KismetSystemLibrary.Delay` 0.1)
              (`|SpawnActorFromClass` "/Game/Characters/AI/AI_golem/BP_Golem_Rock_Projectile.BP_Golem_Rock_Projectile_C" (`KismetMathLibrary.MakeTransform` (+ (+ (`SceneComponent.K2_GetComponentLocation` (`self.ThrowPoint`)) (0.0 0.0 30.0)) (* (`KismetMathLibrary.GetForwardVector` _returnvalue) (100.0 100.0 100.0))) _returnvalue) "Undefined" "OverrideRootScale" null null)
              (`KismetSystemLibrary.PrintString` "Golem is throwing")
              (`KismetSystemLibrary.Delay` 2.0)
              (set `self.Max Walk Speed` 200.0)
              (`BlackboardComponent.SetValueAsBool` (`self.BlackboardRef`) "isAttacking" false)
              (set `self.isChasingPlayer` true)
              (set `self.isAttacking` false)
              (goto _label_2 :!via `Reset`))))))))

(event `self.awakeCollision.OnComponentBeginOverlap`
  (params (OverlappedComponent :type "PrimitiveComponent Object Reference") (OtherActor :type "Actor Object Reference") (OtherComp :type "PrimitiveComponent Object Reference") (OtherBodyIndex :type Integer) (bFromSweep :type Boolean) (SweepResult :type "HitResult Structure (by ref)"))
  (cast `/Game/ThirdPerson/Blueprints/BP_ThirdPersonCharacter_NewBase` OtherActor)
  (`KismetSystemLibrary.Delay` 1.0)
  (`BlackboardComponent.SetValueAsBool` (`self.BlackboardRef`) "isAsleep" false)
  (`KismetSystemLibrary.PrintString` "Golem is AWAKE")
  (set `self.isAwake` true)
  (set `self.isChasingPlayer` true)
  (`BlackboardComponent.SetValueAsBool` (`self.BlackboardRef`) "hasSeenPlayer" true)
  (`BlackboardComponent.SetValueAsBool` (`self.BlackboardRef`) "isRoaming" false))

(event `self.PawnSensing.OnSeePawn`
  (params (Pawn :type "Pawn Object Reference"))
  (if (`self.isAwake`)
    (cast `/Game/ThirdPerson/Blueprints/BP_ThirdPersonCharacter_NewBase` Pawn)
    (set `self.isChasingPlayer` true)
    (`BlackboardComponent.SetValueAsBool` (`self.BlackboardRef`) "hasSeenPlayer" true)
    (`BlackboardComponent.SetValueAsBool` (`self.BlackboardRef`) "isRoaming" false)
    (`KismetSystemLibrary.Delay` (`self.chaseTime`))
    (`BlackboardComponent.SetValueAsBool` (`self.BlackboardRef`) "isRoaming" true)
    (`BlackboardComponent.SetValueAsBool` (`self.BlackboardRef`) "hasSeenPlayer" false)))

(event `self.CapsuleComponent.OnComponentBeginOverlap`
  (params (OverlappedComponent :type "PrimitiveComponent Object Reference") (OtherActor :type "Actor Object Reference") (OtherComp :type "PrimitiveComponent Object Reference") (OtherBodyIndex :type Integer) (bFromSweep :type Boolean) (SweepResult :type "HitResult Structure (by ref)"))
  (bind _asbp_projectile_dark (cast `/Game/Blueprints/Projectiles/BP_Projectile_Dark` OtherActor))
  (bind _asbp_third_person_character_new_base (cast `/Game/ThirdPerson/Blueprints/BP_ThirdPersonCharacter_NewBase` (`GameplayStatics.GetPlayerCharacter` 0)))
  (`/Engine/EditorBlueprintResources/StandardMacros.DoOnce` false :!label _label_3
    (:`Completed`
      (set `self.health` (- (`self.health`) (`/Game/ThirdPerson/Blueprints/BP_ThirdPersonCharacter_NewBase.damage` _asbp_third_person_character_new_base)))
      (set `self.isChasingPlayer` true)
      (`BlackboardComponent.SetValueAsBool` (`self.BlackboardRef`) "hasSeenPlayer" true)
      (`self.K2_DestroyActor` _asbp_projectile_dark)
      (`KismetSystemLibrary.Delay` 0.1)
      (goto _label_3 :!via `Reset`))))

(fn `UserConstructionScript`
  (`parent.UserConstructionScript`))