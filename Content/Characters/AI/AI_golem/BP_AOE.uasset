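; Short-lived area-of-effect actor in the golem AI folder that damages what its sphere collision overlaps, then destroys itself one second after spawning.
; Overlapping non-golem Enemy1_BP actors are marked dead, while golems are left untouched.
; Any other overlap makes player 0's character jump and lose one health, without checking that the overlapping actor is the player.
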(event `self.ReceiveBeginPlay`
  (`KismetSystemLibrary.Delay` 1.0)
  (`self.K2_DestroyActor`))

(event `self.SphereCollision.OnComponentBeginOverlap`
  (params (OverlappedComponent :type "PrimitiveComponent Object Reference") (OtherActor :type "Actor Object Reference") (OtherComp :type "PrimitiveComponent Object Reference") (OtherBodyIndex :type Integer) (bFromSweep :type Boolean) (SweepResult :type "HitResult Structure (by ref)"))
  (bind _asenemy_1_bp (cast `/Game/Characters/AI/AI_Master/Enemy1_BP` OtherActor)
    (:`then`
      (if (not (`/Game/Characters/AI/AI_Master/Enemy1_BP.isGolem` _asenemy_1_bp))
        (set `/Game/Characters/AI/AI_Master/Enemy1_BP.isDead` true _asenemy_1_bp)))
    (:`CastFailed`
      (bind _asbp_third_person_character_new_base (cast `/Game/ThirdPerson/Blueprints/BP_ThirdPersonCharacter_NewBase` (`GameplayStatics.GetPlayerCharacter` 0)))
      (`Character.Jump` _asbp_third_person_character_new_base)
      (bind _result (`/Engine/EditorBlueprintResources/StandardMacros.DecrementFloat` (`/Game/ThirdPerson/Blueprints/BP_ThirdPersonCharacter_NewBase.playerHealth` _asbp_third_person_character_new_base))
        (:`  `
          (set `/Game/ThirdPerson/Blueprints/BP_ThirdPersonCharacter_NewBase.playerHealth` _result _asbp_third_person_character_new_base))))))

(fn `UserConstructionScript`)