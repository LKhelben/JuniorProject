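; Troll AI enemy that senses and attacks the player or Golems, driving its behavior through Blackboard flags.
; Pawn sensing sets seen flags and halts roaming, then restores roaming after a chase delay.
; AttackPlayer sphere-traces ahead, damages only Golems directly, and triggers a montage call before clearing the attack flag.
; Light projectile overlaps reduce the troll's Health, switch its target to the player and destroy the projectile.
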(event `self.Attack Player`
  (bind _returnvalue (`self.K2_GetActorLocation`))
  ;[1 0.6458 0.6458] Attacking Player            https://www.youtube.com/watch?v=LL9hpaSLD5g&ab_channel=GorkaGames
  (if (not (`self.isDead`))
    (`/Engine/EditorBlueprintResources/StandardMacros.DoOnce` false :!label _label
      (:`Completed`
        (bind (_outhit _returnvalue_2) (`KismetSystemLibrary.SphereTraceSingleForObjects` :`Start` _returnvalue :`End` (+ _returnvalue (* (`KismetMathLibrary.GetForwardVector` (`self.K2_GetActorRotation`)) 250.0)) :`Radius` 120.0 :`ObjectTypes` (`|MakeArray` "ObjectTypeQuery3" :!type "EObjectTypeQuery Enum") :`DrawDebugType` "ForDuration" :`bIgnoreSelf` false))
        (if _returnvalue_2
          (`KismetSystemLibrary.PrintString` "Enemy Attacking")
          (bind (_bblockinghit _binitialoverlap _time _distance _location _impactpoint _normal _impactnormal _physmat _hitactor) (`GameplayStatics.BreakHitResult` _outhit))
          (cast `/Game/ThirdPerson/Blueprints/BP_ThirdPersonCharacter_NewBase_Phil` _hitactor
            (:`then`
              _)
            (:`CastFailed`
              (bind _asgolem_bp (cast `/Game/Characters/AI/AI_golem/Golem_BP` _hitactor))
              (set `/Game/Characters/AI/AI_Master/Enemy1_BP.health` (- (`/Game/Characters/AI/AI_Master/Enemy1_BP.health` _asgolem_bp) 1.0) _asgolem_bp)))
          (`self.PlayAnimMontage` null) ; https://youtu.be/LL9hpaSLD5g?t=600
          (`KismetSystemLibrary.Delay` 1.0)
          (`BlackboardComponent.SetValueAsBool` (`self.BlackboardRef`) "isAttacking" false)
          (goto _label :!via `Reset`))))))

(event `self.CapsuleComponent.OnComponentBeginOverlap`
  (params (OverlappedComponent :type "PrimitiveComponent Object Reference") (OtherActor :type "Actor Object Reference") (OtherComp :type "PrimitiveComponent Object Reference") (OtherBodyIndex :type Integer) (bFromSweep :type Boolean) (SweepResult :type "HitResult Structure (by ref)"))
  (bind _asbp_projectile_light (cast `/Game/Blueprints/Projectiles/BP_Projectile_Light` OtherActor))
  (set `self.health` (- (`self.health`) 1.0))
  (set `self.isChasingPlayer` true)
  (set `self.isChasingGolem` false)
  (`BlackboardComponent.SetValueAsBool` (`self.BlackboardRef`) "hasSeenPlayer" true)
  (`BlackboardComponent.SetValueAsBool` (`self.BlackboardRef`) "hasSeenGolem" false)
  (`self.K2_DestroyActor` _asbp_projectile_light))

(event `self.PawnSensing.OnSeePawn`
  (params (Pawn :type "Pawn Object Reference"))
  (cast `/Game/ThirdPerson/Blueprints/BP_ThirdPersonCharacter_NewBase_Phil` Pawn
    (:`then`
      (set `self.isChasingPlayer` true)
      (set `self.isChasingGolem` false)
      (`BlackboardComponent.SetValueAsBool` (`self.BlackboardRef`) "hasSeenPlayer" true)
      (`BlackboardComponent.SetValueAsBool` (`self.BlackboardRef`) "hasSeenGolem" false))
    (:`CastFailed`
      (cast `/Game/Characters/AI/AI_golem/Golem_BP` Pawn)
      (set `self.isChasingGolem` true)
      (`BlackboardComponent.SetValueAsBool` (`self.BlackboardRef`) "hasSeenGolem" true)
      (`KismetSystemLibrary.PrintString` "Troll see Golem")))
  (`BlackboardComponent.SetValueAsBool` (`self.BlackboardRef`) "isRoaming" false)
  (`KismetSystemLibrary.Delay` (`self.chaseTime`))
  (`BlackboardComponent.SetValueAsBool` (`self.BlackboardRef`) "isRoaming" true)
  (`BlackboardComponent.SetValueAsBool` (`self.BlackboardRef`) "hasSeenPlayer" false)
  (`BlackboardComponent.SetValueAsBool` (`self.BlackboardRef`) "hasSeenGolem" false))

(fn `UserConstructionScript`
  (`parent.UserConstructionScript`))