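; Enemy AI character that drives Blackboard states, attacks, and drops random coins on death.
; Tick flags isAttacking when the chased player, troll or golem is within range, and sets IsDead at zero health.
; Death ragdolls the mesh, spawns coins weighted toward bronze, then destroys the actor after a delay.
; ChargeAttack sphere-traces ahead for the player before calling a montage; sight and AttackPlayer events are empty, their older logic disconnected.
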(event `self.ReceiveBeginPlay`
  (set `self.BlackboardRef` (`AIBlueprintHelperLibrary.GetBlackboard` (`AIBlueprintHelperLibrary.GetAIController` self)))
  (set `CharacterMovementComponent.MaxWalkSpeed` (`self.Max Walk Speed`) (`self.CharacterMovement`))
  (`BlackboardComponent.SetValueAsBool` (`self.BlackboardRef`) "isRoaming" true))

(event `self.ReceiveTick`
  (params (DeltaSeconds :type "Float (single-precision)"))
  (bind _silvercoin (`self.silverCoin`))
  (bind _bronzecoin (`self.bronzeCoin`))
  (bind _returnvalue (`SceneComponent.K2_GetComponentToWorld` (`self.SpawnItems`)))
  (`|ExecutionSequence`
    (:`then_0`
      (if (`self.isDead`)
        (`MovementComponent.StopMovementImmediately` (`self.CharacterMovement`))
        (`PrimitiveComponent.SetSimulatePhysics` (`self.Mesh`) true)
        (`/Engine/EditorBlueprintResources/StandardMacros.DoOnce` false
          (:`Completed`
            (for _ (range (+ (`KismetMathLibrary.RandomIntegerInRange` 1 (`self.MaxNumberOfItems`)) 1))
              (`|SpawnActorFromClass` (select `int` (`KismetMathLibrary.RandomIntegerInRange` 0 10) :`0` (`self.goldCoin`) :`1` _silvercoin :`2` _silvercoin :`3` _silvercoin :`4` _bronzecoin :`5` _bronzecoin :`6` _bronzecoin :`7` _bronzecoin :`8` _bronzecoin :`9` _bronzecoin :`10` _bronzecoin :!type "Actor Class Reference") (`KismetMathLibrary.MakeTransform` (`KismetMathLibrary.MakeVector` (+ (.x (.location _returnvalue)) (`KismetMathLibrary.RandomFloatInRange` -25.0 50.0)) (+ (.y (.location _returnvalue)) (`KismetMathLibrary.RandomFloatInRange` -25.0 50.0)) (.z (.location _returnvalue)))) "Undefined" "OverrideRootScale" null null)
              (`KismetSystemLibrary.Delay` 1.0)
              (`self.K2_DestroyActor`))))))
    (:`then_1`
      (if (`self.isChasingPlayer`)
        (bind _asbp_third_person_character_new_base (cast `/Game/ThirdPerson/Blueprints/Broken_BP_ThirdPersonCharacter_NewBase` (`GameplayStatics.GetPlayerCharacter` 0)))
        (if (> (`self.minimumDistanceToAttack`) (`self.GetDistanceTo` _asbp_third_person_character_new_base))
          (`BlackboardComponent.SetValueAsBool` (`self.BlackboardRef`) "isAttacking" true))
        (elif (`self.isChasingTroll`)
          (bind _returnvalue_2 (`GameplayStatics.GetActorOfClass` "/Game/Characters/AI/AI_troll/Troll_BP.Troll_BP_C"))
          (if (> (`self.minimumDistanceToAttack`) (`self.GetDistanceTo` _returnvalue_2))
            (`BlackboardComponent.SetValueAsBool` (`self.BlackboardRef`) "isAttacking" true))
          (elif (`self.isChasingGolem`)
            (bind _returnvalue_3 (`GameplayStatics.GetActorOfClass` "/Game/Characters/AI/AI_golem/Golem_BP.Golem_BP_C"))
            (if (> (`self.minimumDistanceToAttack`) (`self.GetDistanceTo` _returnvalue_3))
              (`BlackboardComponent.SetValueAsBool` (`self.BlackboardRef`) "isAttacking" true))))))
    (:`then_2`
      (if (<= (`self.health`) 0.0)
        (set `self.isDead` true)))))

(event `self.PawnSensing.OnSeePawn`
  (params (Pawn :type "Pawn Object Reference"))
  ;[1 1 1] Detects Player       https://www.youtube.com/watch?v=QJuaB2V79mU&ab_channel=GorkaGames
)

(event `Attack Player`
  ;[1 0.6458 0.6458] Attacking Player            https://www.youtube.com/watch?v=LL9hpaSLD5g&ab_channel=GorkaGames
)

(event `Charge Attack`
  (bind _returnvalue (`self.K2_GetActorLocation`))
  ;[1 0.6458 0.6458] Charge Attacking Player            https://www.youtube.com/watch?v=LL9hpaSLD5g&ab_channel=GorkaGames
  (bind (_outhit _returnvalue_2) (`KismetSystemLibrary.SphereTraceSingleForObjects` :`Start` _returnvalue :`End` (+ _returnvalue (* (`KismetMathLibrary.GetForwardVector` (`self.K2_GetActorRotation`)) 250.0)) :`Radius` 120.0 :`ObjectTypes` (`|MakeArray` "ObjectTypeQuery3" :!type "EObjectTypeQuery Enum") :`DrawDebugType` "ForDuration"))
  (if _returnvalue_2
    (cast `/Game/ThirdPerson/Blueprints/Broken_BP_ThirdPersonCharacter_NewBase` (`.HitActor` (`GameplayStatics.BreakHitResult` _outhit)))
    (`self.PlayAnimMontage` null) ; https://youtu.be/LL9hpaSLD5g?t=600
  ))

(fn `UserConstructionScript`)