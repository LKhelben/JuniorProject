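; Slime enemy AI character that chases the player on sight and fires slime projectiles.
; Pawn sensing flags the player as seen on the blackboard, switching off roaming for a set chase time before restoring it.
; AttackPlayer turns the living slime toward the player, waits briefly, spawns a projectile ahead of the shoot point, then clears the attacking flag.
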(event `self.ReceiveBeginPlay`
  (`parent.ReceiveBeginPlay`))

(event `self.Attack Player`
  (bind _returnvalue (`self.GetControlRotation`))
  (bind (_returnvalue_roll _returnvalue_pitch _returnvalue_yaw) (`KismetMathLibrary.BreakRotator` (`KismetMathLibrary.RInterpTo` (`self.K2_GetActorRotation`) (`KismetMathLibrary.FindLookAtRotation` (`self.K2_GetActorLocation`) (`self.K2_GetActorLocation` (`GameplayStatics.GetPlayerCharacter` 0))) (`GameplayStatics.GetWorldDeltaSeconds`) 50.0)))
  (if (not (`self.isDead`))
    (`self.K2_SetActorRotation` (`KismetMathLibrary.MakeRotator` 0.0 0.0 _returnvalue_yaw))
    (`KismetSystemLibrary.Delay` 0.5)
    (`KismetSystemLibrary.PrintString` "Shooting")
    (`|SpawnActorFromClass` "/Game/Characters/AI/AI_slime/BP_Slime_Projectile.BP_Slime_Projectile_C" (`KismetMathLibrary.MakeTransform` (+ (+ (`SceneComponent.K2_GetComponentLocation` (`self.ShootPos`)) (0.0 0.0 30.0)) (* (`KismetMathLibrary.GetForwardVector` _returnvalue) (100.0 100.0 100.0))) _returnvalue) "Undefined" "OverrideRootScale" null null)
    (`BlackboardComponent.SetValueAsBool` (`self.BlackboardRef`) "isAttacking" false)))

(event `self.PawnSensing.OnSeePawn`
  (params (Pawn :type "Pawn Object Reference"))
  (cast `/Game/ThirdPerson/Blueprints/BP_ThirdPersonCharacter_NewBase_Phil` Pawn)
  (set `self.isChasingPlayer` true)
  (`BlackboardComponent.SetValueAsBool` (`self.BlackboardRef`) "hasSeenPlayer" true)
  (`BlackboardComponent.SetValueAsBool` (`self.BlackboardRef`) "isRoaming" false)
  (`KismetSystemLibrary.Delay` (`self.chaseTime`))
  (`BlackboardComponent.SetValueAsBool` (`self.BlackboardRef`) "isRoaming" true)
  (`BlackboardComponent.SetValueAsBool` (`self.BlackboardRef`) "hasSeenPlayer" false))

(fn `UserConstructionScript`
  (`parent.UserConstructionScript`))