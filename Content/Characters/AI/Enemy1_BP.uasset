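; Enemy1_BP is an AI enemy character that detects the player and performs melee attack checks.
; Pawn sensing sets the hasSeenPlayer Blackboard key when it sees the third-person player character.
; AttackPlayer and ChargeAttack events run identical forward sphere traces with debug drawing, calling PlayAnimMontage on a player hit.
; No damage is applied here, and the direct AIMoveTo follow logic is left unconnected.
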(event `self.ReceiveBeginPlay`)

(event `self.PawnSensing.OnSeePawn`
  (params (Pawn :type "Pawn Object Reference"))
  ;[1 1 1] Detects Player       https://www.youtube.com/watch?v=QJuaB2V79mU&ab_channel=GorkaGames
  (cast `/Game/ThirdPerson/Blueprints/BP_ThirdPersonCharacter_NewBase` Pawn) ; Detects Player
  (`BlackboardComponent.SetValueAsBool` (`AIBlueprintHelperLibrary.GetBlackboard` (`AIBlueprintHelperLibrary.GetAIController` self)) "hasSeenPlayer" true))

(event `Attack Player`
  (bind _returnvalue (`self.K2_GetActorLocation`))
  ;[1 0.6458 0.6458] Attacking Player            https://www.youtube.com/watch?v=LL9hpaSLD5g&ab_channel=GorkaGames
  (bind (_outhit _returnvalue_2) (`KismetSystemLibrary.SphereTraceSingleForObjects` :`Start` _returnvalue :`End` (+ _returnvalue (* (`KismetMathLibrary.GetForwardVector` (`self.K2_GetActorRotation`)) 250.0)) :`Radius` 120.0 :`ObjectTypes` (`|MakeArray` "ObjectTypeQuery3" :!type "EObjectTypeQuery Enum") :`DrawDebugType` "ForDuration"))
  (if _returnvalue_2
    (cast `/Game/ThirdPerson/Blueprints/BP_ThirdPersonCharacter_NewBase` (`.HitActor` (`GameplayStatics.BreakHitResult` _outhit)))
    (`self.PlayAnimMontage` null) ; https://youtu.be/LL9hpaSLD5g?t=600
  ))

(event `Charge Attack`
  (bind _returnvalue (`self.K2_GetActorLocation`))
  ;[1 0.6458 0.6458] Charge Attacking Player            https://www.youtube.com/watch?v=LL9hpaSLD5g&ab_channel=GorkaGames
  (bind (_outhit _returnvalue_2) (`KismetSystemLibrary.SphereTraceSingleForObjects` :`Start` _returnvalue :`End` (+ _returnvalue (* (`KismetMathLibrary.GetForwardVector` (`self.K2_GetActorRotation`)) 250.0)) :`Radius` 120.0 :`ObjectTypes` (`|MakeArray` "ObjectTypeQuery3" :!type "EObjectTypeQuery Enum") :`DrawDebugType` "ForDuration"))
  (if _returnvalue_2
    (cast `/Game/ThirdPerson/Blueprints/BP_ThirdPersonCharacter_NewBase` (`.HitActor` (`GameplayStatics.BreakHitResult` _outhit)))
    (`self.PlayAnimMontage` null) ; https://youtu.be/LL9hpaSLD5g?t=600
  ))

(fn `UserConstructionScript`)