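; Master coin pickup that adds its Value to the third-person character's Currency on touch, then destroys itself.
; At BeginPlay it either floats or drops with physics, per CanFloat, while timelines spin and bob the coin mesh.
; When the player enters the attraction radius, physics turns off and a timeline moves the actor toward the player using VInterpTo at AttractionSpeed plus a track offset.
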(event `self.ReceiveBeginPlay`
  (bind _base (`self.Base`))
  (bind (_relativelocation_x _relativelocation_y) (`KismetMathLibrary.BreakVector` (`SceneComponent.RelativeLocation` (`self.Coin`))))
  (`|ExecutionSequence`
    (:`then_0`
      (if (`self.canFloat`)
        (`PrimitiveComponent.SetEnableGravity` _base false)
        (else
          (`PrimitiveComponent.SetSimulatePhysics` _base true)
          (`PrimitiveComponent.SetEnableGravity` _base true))))
    (:`then_1`
      (bind (_direction _rotator) (`Timeline|Rotation` :!via `PlayFromStart`)
        (:`Update`
          (`SceneComponent.K2_SetRelativeRotation` (`self.Coin`) (`KismetMathLibrary.RLerp` (struct :`Roll` -90.0) (struct :`Pitch` 360.0 :`Yaw` 360.0 :`Roll` -90.0) _rotator) false false))))
    (:`then_2`
      (bind (_direction_2 _updown) (`Timeline|Location`)
        (:`Update`
          (`SceneComponent.K2_SetRelativeLocation` (`self.Coin`) (`KismetMathLibrary.MakeVector` _relativelocation_x _relativelocation_y _updown) false false))))))

(event `self.ReceiveTick`
  (params (DeltaSeconds :type "Float (single-precision)")))

(event `self.Attraction_radius.OnComponentBeginOverlap`
  (params (OverlappedComponent :type "PrimitiveComponent Object Reference") (OtherActor :type "Actor Object Reference") (OtherComp :type "PrimitiveComponent Object Reference") (OtherBodyIndex :type Integer) (bFromSweep :type Boolean) (SweepResult :type "HitResult Structure (by ref)"))
  (if (== OtherActor (`GameplayStatics.GetPlayerCharacter` 0))
    (`PrimitiveComponent.SetSimulatePhysics` (`self.Base`) false)
    (`KismetSystemLibrary.PrintString` "Physics disabled" false false)
    (bind (_direction _newtrack_0) (`Timeline|Attraction` :!via `PlayFromStart`)
      (:`Update`
        (`self.K2_SetActorLocation` (+ _newtrack_0 (`KismetMathLibrary.VInterpTo` (.location (`self.GetTransform`)) (`self.K2_GetActorLocation` (`GameplayStatics.GetPlayerCharacter` 0)) (`GameplayStatics.GetWorldDeltaSeconds`) (`self.attractionSpeed`))))))))

(event `self.Coin.OnComponentBeginOverlap`
  (params (OverlappedComponent :type "PrimitiveComponent Object Reference") (OtherActor :type "Actor Object Reference") (OtherComp :type "PrimitiveComponent Object Reference") (OtherBodyIndex :type Integer) (bFromSweep :type Boolean) (SweepResult :type "HitResult Structure (by ref)"))
  (bind _returnvalue (`GameplayStatics.GetPlayerCharacter` 0))
  (if (== OtherActor _returnvalue)
    (bind _asbp_third_person_character_new_base (cast `/Game/ThirdPerson/Blueprints/BP_ThirdPersonCharacter_NewBase` _returnvalue))
    (set `/Game/ThirdPerson/Blueprints/BP_ThirdPersonCharacter_NewBase.currency` (+ (`/Game/ThirdPerson/Blueprints/BP_ThirdPersonCharacter_NewBase.currency` _asbp_third_person_character_new_base) (`self.value`)) _asbp_third_person_character_new_base)
    (`self.K2_DestroyActor`)))

(fn `UserConstructionScript`)