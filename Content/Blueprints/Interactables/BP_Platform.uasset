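; BP_Platform is an interactable platform that moves vertically through MovePlatformUp and MovePlatformDown events.
; Each event plays its own timeline, lerping the Platform component's relative Z toward a fixed offset from its current position, so movement accumulates every update.
; IsMoving blocks new moves during playback.
; On completion, IsFinished is set for a one-second delay, during which Tick clears IsMoving.
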(event `self.ReceiveTick`
  (params (DeltaSeconds :type "Float (single-precision)"))
  (if (`self.isFinished`)
    (set `self.isMoving` false)))

(event `MovePlatformUp`
  (bind _returnvalue_location (`KismetMathLibrary.BreakTransform` (`SceneComponent.GetRelativeTransform` (`self.Platform`))))
  (if (not (`self.isMoving`))
    (bind (_direction _open_track) (`Timeline|Move Platform Timeline` :!via `PlayFromStart`)
      (:`Update`
        (set `self.isMoving` true)
        (`SceneComponent.K2_SetRelativeLocation` (`self.Platform`) (`KismetMathLibrary.VLerp` _returnvalue_location (+ _returnvalue_location (0.0 0.0 50.0)) _open_track) false false))
      (:`Finished`
        (set `self.isFinished` true)
        (`KismetSystemLibrary.Delay` 1.0 :!label _label)
        (set `self.isFinished` false)))))

(event `MovePlatformDown`
  (bind _returnvalue_location (`KismetMathLibrary.BreakTransform` (`SceneComponent.GetRelativeTransform` (`self.Platform`))))
  (if (not (`self.isMoving`))
    (bind (_direction _open_track) (`Timeline|Timeline_0` :!via `PlayFromStart`)
      (:`Update`
        (set `self.isMoving` true)
        (`SceneComponent.K2_SetRelativeLocation` (`self.Platform`) (`KismetMathLibrary.VLerp` _returnvalue_location (- _returnvalue_location (0.0 0.0 50.0)) _open_track) false false))
      (:`Finished`
        (set `self.isFinished` true)
        (goto _label)))))

(fn `UserConstructionScript`)