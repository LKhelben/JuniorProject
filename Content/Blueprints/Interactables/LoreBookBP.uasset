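; Interactable lore book actor that lets the player open and close a journal by pressing E while near it.
; Box overlap with the third-person character caches that character and enables input on the actor; leaving disables it.
; E toggles the character's IsReading flag, creating a Book widget with this book's number or removing it from the viewport.
; A DoOnce guards widget creation and resets when the widget is removed.
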(event `Key|E`
  (params (Key :type "Key Structure"))
  ;[0.3333 0 0.02353] Allows the player to read the books
  (:`Pressed`
    (if (`/Game/ThirdPerson/Blueprints/BP_ThirdPersonCharacter_NewBase.isReading` (stale `self.Box.OnComponentBeginOverlap` _asbp_third_person_character_new_base))
      (set `/Game/ThirdPerson/Blueprints/BP_ThirdPersonCharacter_NewBase.isReading` false (stale `self.Box.OnComponentBeginOverlap` _asbp_third_person_character_new_base))
      ;[0.3333 0 0.02353] Adds and removes book to and from viewport
      (`/Engine/EditorBlueprintResources/StandardMacros.IsValid` (stale _returnvalue)
        (:`Is Valid`
          (`Widget.RemoveFromParent` (stale _returnvalue))
          (goto _label :!via `Reset`)))
      (else
        (set `/Game/ThirdPerson/Blueprints/BP_ThirdPersonCharacter_NewBase.isReading` true (stale `self.Box.OnComponentBeginOverlap` _asbp_third_person_character_new_base))
        (`/Engine/EditorBlueprintResources/StandardMacros.DoOnce` false :!label _label
          (:`Completed`
            (bind _returnvalue (`|CreateWidget` "/Game/Assets/Lore_Books/Book.Book_C"))
            (set `/Game/Assets/Lore_Books/Book.JournalNumber` (`self.Book Number`) _returnvalue)
            (`UserWidget.AddToViewport` _returnvalue 0)))))))

(event `self.Box.OnComponentBeginOverlap`
  (params (OverlappedComponent :type "PrimitiveComponent Object Reference") (OtherActor :type "Actor Object Reference") (OtherComp :type "PrimitiveComponent Object Reference") (OtherBodyIndex :type Integer) (bFromSweep :type Boolean) (SweepResult :type "HitResult Structure (by ref)"))
  ;[0.3333 0 0.02353] Allows the player to read the books
  (bind _asbp_third_person_character_new_base (cast `/Game/ThirdPerson/Blueprints/BP_ThirdPersonCharacter_NewBase` OtherActor))
  (`self.EnableInput` (`GameplayStatics.GetPlayerController` 0)))

(event `self.Box.OnComponentEndOverlap`
  (params (OverlappedComponent :type "PrimitiveComponent Object Reference") (OtherActor :type "Actor Object Reference") (OtherComp :type "PrimitiveComponent Object Reference") (OtherBodyIndex :type Integer))
  ;[0.3333 0 0.02353] Allows the player to read the books
  (cast `/Game/ThirdPerson/Blueprints/BP_ThirdPersonCharacter_NewBase` OtherActor)
  (`self.DisableInput` (`GameplayStatics.GetPlayerController` 0)))

(fn `UserConstructionScript`)