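; A breakable wooden crate that bursts into debris and coins when a BP_Projectile_Dark or Enemy1_BP overlaps its collision box.
; A random-length loop, capped by MaxNumberOfItems, spawns two broken-wood pieces, plays a break sound and drops a coin on each pass.
; Coin type is a weighted random pick favouring bronze over silver and gold, scattered in X/Y around SpawnPoint.
; The crate destroys itself once the loop finishes.
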(event `self.CollisionBox.OnComponentBeginOverlap`
  (params (OverlappedComponent :type "PrimitiveComponent Object Reference") (OtherActor :type "Actor Object Reference") (OtherComp :type "PrimitiveComponent Object Reference") (OtherBodyIndex :type Integer) (bFromSweep :type Boolean) (SweepResult :type "HitResult Structure (by ref)"))
  (bind _silvercoin (`self.silverCoin`))
  (bind _bronzecoin (`self.bronzeCoin`))
  (bind _returnvalue (`SceneComponent.K2_GetComponentToWorld` (`self.Spawn Point`)))
  (bind _returnvalue_2 (`KismetMathLibrary.Conv_VectorToTransform` (`SceneComponent.K2_GetComponentLocation` (`self.Spawn Point`))))
  (cast `/Game/Blueprints/Projectiles/BP_Projectile_Dark` OtherActor
    (:`then`
      _)
    (:`CastFailed`
      (cast `/Game/Characters/AI/AI_Master/Enemy1_BP` OtherActor)))
  (for _ (range (+ (`KismetMathLibrary.RandomIntegerInRange` 1 (`self.MaxNumberOfItems`)) 1))
    (`|SpawnActorFromClass` "/Game/Blueprints/Interactables/BP_BrokenWoodenPartsA.BP_BrokenWoodenPartsA_C" _returnvalue_2 "Undefined" "OverrideRootScale" null null)
    (`|SpawnActorFromClass` "/Game/Blueprints/Interactables/BP_BrokenWoodenPartsB.BP_BrokenWoodenPartsB_C" _returnvalue_2 "Undefined" "OverrideRootScale" null null)
    (`GameplayStatics.PlaySound2D` "/Game/SFX/woodBreak.woodBreak" 1.0 1.0 0.0 null null)
    (`|SpawnActorFromClass` (select `int` (`KismetMathLibrary.RandomIntegerInRange` 0 10) :`0` (`self.goldCoin`) :`1` _silvercoin :`2` _silvercoin :`3` _silvercoin :`4` _bronzecoin :`5` _bronzecoin :`6` _bronzecoin :`7` _bronzecoin :`8` _bronzecoin :`9` _bronzecoin :`10` _bronzecoin :!type "Actor Class Reference") (`KismetMathLibrary.MakeTransform` (`KismetMathLibrary.MakeVector` (+ (.x (.location _returnvalue)) (`KismetMathLibrary.RandomFloatInRange` -25.0 50.0)) (+ (.y (.location _returnvalue)) (`KismetMathLibrary.RandomFloatInRange` -25.0 50.0)) (.z (.location _returnvalue)))) "Undefined" "OverrideRootScale" null null))
  (`self.K2_DestroyActor`))

(fn `UserConstructionScript`)