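; Interactable button that raises and lowers the BP_Platform actors whose ObjectValue matches its ButtonValue.
; A box overlap shows an interact widget to the player character unless IsUsed is set, and hides it on exit.
; ActivateObject scans all platforms and, for each idle match, plays a timeline press animation and calls move up or down through one shared FlipFlop, so successive calls alternate.
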(event `self.BoxCollision.OnComponentBeginOverlap`
  (params (OverlappedComponent :type "PrimitiveComponent Object Reference") (OtherActor :type "Actor Object Reference") (OtherComp :type "PrimitiveComponent Object Reference") (OtherBodyIndex :type Integer) (bFromSweep :type Boolean) (SweepResult :type "HitResult Structure (by ref)"))
  (cast `/Game/ThirdPerson/Blueprints/BP_ThirdPersonCharacter_NewBase` OtherActor)
  (if (`self.isUsed`)
    (`SceneComponent.SetHiddenInGame` (`self.Interact Widget`) true false :!label _label)
    (else
      (`SceneComponent.SetHiddenInGame` (`self.Interact Widget`) false false))))

(event `self.BoxCollision.OnComponentEndOverlap`
  (params (OverlappedComponent :type "PrimitiveComponent Object Reference") (OtherActor :type "Actor Object Reference") (OtherComp :type "PrimitiveComponent Object Reference") (OtherBodyIndex :type Integer))
  (cast `/Game/ThirdPerson/Blueprints/BP_ThirdPersonCharacter_NewBase` OtherActor)
  (goto _label))

(event `/Game/Blueprints/UI-UX/Object_Interact.Activate Object`
  (bind _outactors (`GameplayStatics.GetAllActorsOfClass` "/Game/Blueprints/Interactables/BP_Platform.BP_Platform_C"))
  (for _array_element _outactors
    (if (== (`/Game/Blueprints/Interactables/BP_Platform.objectValue` _array_element) (`self.buttonValue`))
      (if (not (`/Game/Blueprints/Interactables/BP_Platform.isMoving` _array_element))
        (`self.ButtonAnimation`)
        (`/Engine/EditorBlueprintResources/StandardMacros.FlipFlop`
          (:`A`
            (`/Game/Blueprints/Interactables/BP_Platform.MovePlatformUp` _array_element))
          (:`B`
            (`/Game/Blueprints/Interactables/BP_Platform.MovePlatformDown` _array_element)))))))

(event `ButtonAnimation`
  (bind (_direction _playtrack) (`Timeline|ButtonPress` :!via `PlayFromStart`)
    (:`Update`
      (`SceneComponent.K2_SetRelativeLocation` (`self.Button`) (`KismetMathLibrary.VLerp` (0.0 0.0 0.0) (0.0 -5.0 0.0) _playtrack) false false))))

(fn `UserConstructionScript`)