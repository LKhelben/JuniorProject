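; Interactable loot chest that shows an interaction widget while the player overlaps its box and it is unused.
; ActivateObject works once: it hides the lid and widget and spawns a BP_ChestTop in the lid's place.
; It then spawns a random number of coins scattered around SpawnPoint, weighted toward bronze over silver and gold through repeated Select options.
; A delay in the spawn loop destroys the chest 15 seconds later.
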(event `self.BoxCollision.OnComponentBeginOverlap`
  (params (OverlappedComponent :type "PrimitiveComponent Object Reference") (OtherActor :type "Actor Object Reference") (OtherComp :type "PrimitiveComponent Object Reference") (OtherBodyIndex :type Integer) (bFromSweep :type Boolean) (SweepResult :type "HitResult Structure (by ref)"))
  (cast `/Game/ThirdPerson/Blueprints/BP_PlayerQUYNHS` OtherActor)
  (if (`self.isUsed`)
    (`SceneComponent.SetHiddenInGame` (`self.InteractionWidget`) true false :!label _label)
    (else
      (`SceneComponent.SetHiddenInGame` (`self.InteractionWidget`) false false))))

(event `self.BoxCollision.OnComponentEndOverlap`
  (params (OverlappedComponent :type "PrimitiveComponent Object Reference") (OtherActor :type "Actor Object Reference") (OtherComp :type "PrimitiveComponent Object Reference") (OtherBodyIndex :type Integer))
  (cast `/Game/ThirdPerson/Blueprints/BP_PlayerQUYNHS` OtherActor)
  (goto _label))

(event `/Game/Blueprints/UI-UX/Object_Interact.Activate Object`
  (bind _top (`self.Top`))
  (bind _silvercoin (`self.silverCoin`))
  (bind _bronzecoin (`self.bronzeCoin`))
  (bind _returnvalue (`SceneComponent.K2_GetComponentToWorld` (`self.SpawnPoint`)))
  (if (not (`self.isUsed`))
    (set `self.isUsed` true)
    (`SceneComponent.SetHiddenInGame` _top true false)
    (`SceneComponent.SetHiddenInGame` (`self.InteractionWidget`) true false)
    (`|SpawnActorFromClass` "/Game/Blueprints/Interactables/BP_ChestTOp.BP_ChestTop_C" (`SceneComponent.K2_GetComponentToWorld` _top) "Undefined" "OverrideRootScale" null null)
    (for _ (range (+ (`KismetMathLibrary.RandomIntegerInRange` 1 (`self.MaxNumberOfItems`)) 1))
      (`|SpawnActorFromClass` (select `int` (`KismetMathLibrary.RandomIntegerInRange` 0 10) :`0` (`self.goldCoin`) :`1` _silvercoin :`2` _silvercoin :`3` _silvercoin :`4` _bronzecoin :`5` _bronzecoin :`6` _bronzecoin :`7` _bronzecoin :`8` _bronzecoin :`9` _bronzecoin :`10` _bronzecoin :!type "Actor Class Reference") (`KismetMathLibrary.MakeTransform` (`KismetMathLibrary.MakeVector` (+ (.x (.location _returnvalue)) (`KismetMathLibrary.RandomFloatInRange` -25.0 50.0)) (+ (.y (.location _returnvalue)) (`KismetMathLibrary.RandomFloatInRange` -25.0 50.0)) (.z (.location _returnvalue)))) "Undefined" "OverrideRootScale" null null)
      (`KismetSystemLibrary.Delay` 15.0)
      (`self.K2_DestroyActor`))))

(fn `UserConstructionScript`)