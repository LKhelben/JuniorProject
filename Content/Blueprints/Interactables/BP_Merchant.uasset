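; Merchant NPC that shows an interact prompt and plays ambient voice chatter when the player enters its area.
; ActivateDialogue cuts off the chatter, hides the prompt and player mesh, opens the WD_Merchant widget and plays one of two random Skeebo greetings.
; PlayerAdjustments switches to UI-only mouse input and blends the view to the merchant's shop camera, positioned by the construction script.
; A delayed flag gates chatter replay, though a comment notes it is broken.
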(event `self.ReceiveTick`
  (params (DeltaSeconds :type "Float (single-precision)")))

(event `self.Interact Area.OnComponentBeginOverlap`
  (params (OverlappedComponent :type "PrimitiveComponent Object Reference") (OtherActor :type "Actor Object Reference") (OtherComp :type "PrimitiveComponent Object Reference") (OtherBodyIndex :type Integer) (bFromSweep :type Boolean) (SweepResult :type "HitResult Structure (by ref)"))
  ;[1 1 1] Show Interact
  (cast `/Game/ThirdPerson/Blueprints/BP_PlayerQUYNHS` OtherActor)
  (`SceneComponent.SetHiddenInGame` (`self.Interact`) false false)
  (if (`self.SFX CanTalk `)
    ;[0.7819 0.6036 1] SFX
    ;;[1 1 1] Adventures
    (bind _returnvalue (`AddComponent|NODE_AddAudioComponent-4`))
    (set `self.SVFX RandomConvo` _returnvalue)
    (set `self.SFX CanTalk ` false)
    (if (`self.SFX CutoffTalk`)
      (`AudioComponent.Stop` _returnvalue :!label _label)
      (else
        (`KismetSystemLibrary.Delay` 15.0)
        (set `self.SFX CanTalk ` true) ; doesnt work but its ok bc it would get pretty annoying
      ))))

(event `self.Interact Area.OnComponentEndOverlap`
  (params (OverlappedComponent :type "PrimitiveComponent Object Reference") (OtherActor :type "Actor Object Reference") (OtherComp :type "PrimitiveComponent Object Reference") (OtherBodyIndex :type Integer))
  ;[1 1 1] Show Interact
  (cast `/Game/ThirdPerson/Blueprints/BP_PlayerQUYNHS` OtherActor)
  (`SceneComponent.SetHiddenInGame` (`self.Interact`) true false))

(event `/Game/Blueprints/UI-UX/NPC_Interact.Activate Dialogue`
  ;[0.9098 0.5158 1] VFX
  (`|ExecutionSequence`
    (:`then_0`
      (set `self.SFX CutoffTalk` true)
      (`self.PlayerAdjustments`)
      (`SceneComponent.SetHiddenInGame` (`self.Interact`) true false)
      (bind _asbp_third_person_character_new_base (cast `/Game/ThirdPerson/Blueprints/BP_PlayerQUYNHS` (`GameplayStatics.GetPlayerCharacter` 0)))
      (`SceneComponent.SetHiddenInGame` (`Character.Mesh` _asbp_third_person_character_new_base) true false)
      (bind _returnvalue (`|CreateWidget` "/Game/Blueprints/UI-UX/WD_Merchant.WD_Merchant_C"))
      (`UserWidget.AddToPlayerScreen` _returnvalue 0)
      ;[0.6417 0.5249 1] SFX
      (set `self.SFX Greeting ` (`KismetMathLibrary.RandomIntegerInRange` 0 1))
      ;;[1 1 1] Greeting 1
      (if (== (`self.SFX Greeting `) 0)
        (`GameplayStatics.PlaySound2D` "/Game/SFX/Character/Skeebo/Skeebo_Player_Asks_About_Other_Adventurers.Skeebo_Player_Asks_About_Other_Adventurers" 1.0 1.0 0.0 null null)
        (else
          ;;[1 1 1] Greeting 2
          (if (== (`self.SFX Greeting `) 1)
            (`GameplayStatics.PlaySound2D` "/Game/SFX/Character/Skeebo/Skeebo_Greeting_Line.Skeebo_Greeting_Line" 1.0 1.0 0.0 null null)))))
    (:`then_1`
      (goto _label))))

(event `PlayerAdjustments`
  (bind _returnvalue (`GameplayStatics.GetPlayerController` 0))
  (set `PlayerController.bShowMouseCursor` true _returnvalue)
  (`WidgetBlueprintLibrary.SetInputMode_UIOnlyEx` _returnvalue null)
  (`PlayerController.SetViewTargetWithBlend` (`GameplayStatics.GetPlayerController` 0) (`ActorComponent.GetOwner` (`self.CameraShop`)) 0.0 "VTBlend_Linear" 0.0 false))

(fn `UserConstructionScript`
  (`SceneComponent.K2_SetRelativeTransform` (`self.CameraShop`) (`self.CameraTransform`) false false))