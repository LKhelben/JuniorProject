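; BP_Lever is an interactable lever that the player toggles on and off with the E key while nearby.
; Its Box overlap enables input when the player character enters and disables it on exit.
; A FlipFlop on the key press drives the TIsOn state, with no movement or visual response in this graph.
; BeginPlay caches the player character in TPlayer, which the graph does not otherwise use.
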(event `self.Box.OnComponentBeginOverlap`
  (params (OverlappedComponent :type "PrimitiveComponent Object Reference") (OtherActor :type "Actor Object Reference") (OtherComp :type "PrimitiveComponent Object Reference") (OtherBodyIndex :type Integer) (bFromSweep :type Boolean) (SweepResult :type "HitResult Structure (by ref)"))
  ;[0.3333 0 0.02353] Enables/Disables input when the player is near the lever
  (cast `/Game/ThirdPerson/Blueprints/Broken_BP_ThirdPersonCharacter_NewBase` OtherActor)
  (`self.EnableInput` (`GameplayStatics.GetPlayerController` 0)))

(event `self.Box.OnComponentEndOverlap`
  (params (OverlappedComponent :type "PrimitiveComponent Object Reference") (OtherActor :type "Actor Object Reference") (OtherComp :type "PrimitiveComponent Object Reference") (OtherBodyIndex :type Integer))
  ;[0.3333 0 0.02353] Enables/Disables input when the player is near the lever
  (cast `/Game/ThirdPerson/Blueprints/Broken_BP_ThirdPersonCharacter_NewBase` OtherActor)
  (`self.DisableInput` (`GameplayStatics.GetPlayerController` 0)))

(event `self.ReceiveBeginPlay`
  ;[0.3333 0 0.02353] Sets the value of player
  (bind _aspatterson_bp_third_person_character_new_base (cast `/Game/ThirdPerson/Blueprints/Broken_BP_ThirdPersonCharacter_NewBase` (`GameplayStatics.GetPlayerCharacter` 0)))
  (set `self.tPlayer` _aspatterson_bp_third_person_character_new_base))

(event `Key|E`
  (params (Key :type "Key Structure"))
  ;[0.3333 0 0.02353] Turns the lever on/off when flipped
  (:`Pressed`
    (bind _isa (`/Engine/EditorBlueprintResources/StandardMacros.FlipFlop`)
      (:`A`
        _)
      (:`B`
        _))
    (set `self.tIsOn` _isa)))

(fn `UserConstructionScript`)