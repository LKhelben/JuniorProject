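; Boss door interactable with two leaves that swing open once the player holds all three keys.
; A box overlap casts to the third-person character and calls ActivateObject when its three key flags are set.
; ActivateObject restarts the Rotating timeline, which lerps both leaves toward the same fixed rotation.
; Each update lerps from the current relative rotation rather than a stored start, so motion does not linearly follow the curve.
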(event `self.Activate Object`
  (bind (_returnvalue_location _returnvalue_rotation _returnvalue_scale) (`KismetMathLibrary.BreakTransform` (`SceneComponent.GetRelativeTransform` (`self.leftDoor`))))
  (bind (_returnvalue_location_2 _returnvalue_rotation_2 _returnvalue_scale_2) (`KismetMathLibrary.BreakTransform` (`SceneComponent.GetRelativeTransform` (`self.rightDoor`))))
  (bind (_direction _alpha) (`Timeline|Rotating` :!via `PlayFromStart`)
    (:`Update`
      (`|ExecutionSequence`
        (:`then_0`
          (`SceneComponent.K2_SetRelativeTransform` (`self.rightDoor`) (`KismetMathLibrary.MakeTransform` _returnvalue_location_2 (`KismetMathLibrary.RLerp` _returnvalue_rotation_2 (struct :`Yaw` -95.0) _alpha) _returnvalue_scale_2) false false))
        (:`then_1`
          (`SceneComponent.K2_SetRelativeTransform` (`self.leftDoor`) (`KismetMathLibrary.MakeTransform` _returnvalue_location (`KismetMathLibrary.RLerp` _returnvalue_rotation (struct :`Yaw` -95.0) _alpha) _returnvalue_scale) false false))))))

(event `self.BoxCollision.OnComponentBeginOverlap`
  (params (OverlappedComponent :type "PrimitiveComponent Object Reference") (OtherActor :type "Actor Object Reference") (OtherComp :type "PrimitiveComponent Object Reference") (OtherBodyIndex :type Integer) (bFromSweep :type Boolean) (SweepResult :type "HitResult Structure (by ref)"))
  (bind _asbp_third_person_character_new_base (cast `/Game/ThirdPerson/Blueprints/BP_ThirdPersonCharacter_NewBase` OtherActor))
  (if (and (`/Game/ThirdPerson/Blueprints/BP_ThirdPersonCharacter_NewBase.hasKey01` _asbp_third_person_character_new_base) (`/Game/ThirdPerson/Blueprints/BP_ThirdPersonCharacter_NewBase.hasKey02` _asbp_third_person_character_new_base) (`/Game/ThirdPerson/Blueprints/BP_ThirdPersonCharacter_NewBase.hasKey03` _asbp_third_person_character_new_base))
    (`self.Activate Object`)))

(fn `UserConstructionScript`)