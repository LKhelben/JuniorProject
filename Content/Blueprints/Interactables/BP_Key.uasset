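; BP_Key is a pickup that gives the player character one of three keys when it overlaps the key's box.
; On overlap it casts the other actor to the third-person character, then checks its IsKey01, IsKey02 and IsKey03 flags in order.
; The first true flag sets the matching HasKey boolean on the character and destroys the pickup; with none set, nothing happens.
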(event `self.Box.OnComponentBeginOverlap`
  (params (OverlappedComponent :type "PrimitiveComponent Object Reference") (OtherActor :type "Actor Object Reference") (OtherComp :type "PrimitiveComponent Object Reference") (OtherBodyIndex :type Integer) (bFromSweep :type Boolean) (SweepResult :type "HitResult Structure (by ref)"))
  (bind _asbp_third_person_character_new_base (cast `/Game/ThirdPerson/Blueprints/BP_ThirdPersonCharacter_NewBase_Phil` OtherActor))
  (if (`self.isKey01`)
    (set `/Game/ThirdPerson/Blueprints/BP_ThirdPersonCharacter_NewBase_Phil.hasKey01` true _asbp_third_person_character_new_base)
    (`self.K2_DestroyActor` :!label _label)
    (elif (`self.isKey02`)
      (set `/Game/ThirdPerson/Blueprints/BP_ThirdPersonCharacter_NewBase_Phil.hasKey02` true _asbp_third_person_character_new_base)
      (goto _label)
      (elif (`self.isKey03`)
        (set `/Game/ThirdPerson/Blueprints/BP_ThirdPersonCharacter_NewBase_Phil.hasKey03` true _asbp_third_person_character_new_base)
        (goto _label)))))

(fn `UserConstructionScript`)