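; BP_Platform_2 is an interactable platform that endlessly swings 80 degrees away from level and back on a timed cycle.
; Tick drives a DoOnce-gated sequence that waits Timer seconds, calls DropPlatform, waits again, calls RisePlatform, then resets the gate.
; Each event plays its own timeline, lerping the Platform's relative rotation from its current value toward the target while preserving location and scale.
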(event `self.ReceiveTick`
  (params (DeltaSeconds :type "Float (single-precision)"))
  (`/Engine/EditorBlueprintResources/StandardMacros.DoOnce` false :!label _label
    (:`Completed`
      (`KismetSystemLibrary.Delay` (`self.timer`))
      (`self.DropPlatform`)
      (`KismetSystemLibrary.Delay` (`self.timer`))
      (`self.Rise Platform`)
      (goto _label :!via `Reset`))))

(event `DropPlatform`
  (bind (_returnvalue_location _returnvalue_rotation _returnvalue_scale) (`KismetMathLibrary.BreakTransform` (`SceneComponent.GetRelativeTransform` (`self.Platform`))))
  (bind (_direction _open_track) (`Timeline|Move Platform Timeline` :!via `PlayFromStart`)
    (:`Update`
      (`SceneComponent.K2_SetRelativeTransform` (`self.Platform`) (`KismetMathLibrary.MakeTransform` _returnvalue_location (`KismetMathLibrary.RLerp` _returnvalue_rotation (struct :`Pitch` -80.0) _open_track) _returnvalue_scale) false false))))

(event `Rise Platform`
  (bind (_returnvalue_location _returnvalue_rotation _returnvalue_scale) (`KismetMathLibrary.BreakTransform` (`SceneComponent.GetRelativeTransform` (`self.Platform`))))
  (bind (_direction _open_track) (`Timeline|Timeline_0` :!via `PlayFromStart`)
    (:`Update`
      (`SceneComponent.K2_SetRelativeTransform` (`self.Platform`) (`KismetMathLibrary.MakeTransform` _returnvalue_location (`KismetMathLibrary.RLerp` _returnvalue_rotation (struct) _open_track) _returnvalue_scale) false false))))

(fn `UserConstructionScript`)