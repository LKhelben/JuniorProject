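; BP_Lift is an interactable lift whose Platform moves vertically through externally callable MovePlatformUp and MovePlatformDown events.
; Each event plays its own timeline, lerping every update from the platform's current relative location toward an offset of HeightAmount, so movement accumulates rather than using fixed endpoints.
; AtTop and IsMoving gate requests by position and motion.
; Tick clears IsMoving once IsFinished is set, which a shared delay later resets.
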(event `self.ReceiveTick`
  (params (DeltaSeconds :type "Float (single-precision)"))
  (if (`self.isFinished`)
    (set `self.isMoving` false)))

(event `MovePlatformUp`
  (bind _returnvalue_location (`KismetMathLibrary.BreakTransform` (`SceneComponent.GetRelativeTransform` (`self.Platform`))))
  (if (not (`self.isMoving`))
    (if (not (`self.atTop`))
      (bind (_direction _open_track) (`Timeline|Move Platform Timeline` :!via `PlayFromStart`)
        (:`Update`
          (set `self.isMoving` true)
          (`SceneComponent.K2_SetRelativeLocation` (`self.Platform`) (`KismetMathLibrary.VLerp` _returnvalue_location (+ _returnvalue_location (`KismetMathLibrary.MakeVector` 0.0 0.0 (`self.heightAmount`))) _open_track) false false)
          (set `self.atTop` true))
        (:`Finished`
          (set `self.isFinished` true)
          (`KismetSystemLibrary.Delay` 1.0 :!label _label)
          (set `self.isFinished` false)
          (set `self.isMoving` false))))))

(event `MovePlatformDown`
  (bind _returnvalue_location (`KismetMathLibrary.BreakTransform` (`SceneComponent.GetRelativeTransform` (`self.Platform`))))
  (if (not (`self.isMoving`))
    (if (`self.atTop`)
      (bind (_direction _open_track) (`Timeline|Timeline_0` :!via `PlayFromStart`)
        (:`Update`
          (set `self.isMoving` true)
          (`SceneComponent.K2_SetRelativeLocation` (`self.Platform`) (`KismetMathLibrary.VLerp` _returnvalue_location (- _returnvalue_location (`KismetMathLibrary.MakeVector` 0.0 0.0 (`self.heightAmount`))) _open_track) false false)
          (set `self.atTop` false))
        (:`Finished`
          (set `self.isFinished` true)
          (goto _label))))))

(fn `UserConstructionScript`)