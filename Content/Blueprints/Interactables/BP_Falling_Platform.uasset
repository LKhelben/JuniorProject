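; BP_Falling_Platform is a hinged platform that repeatedly swings down and back up on its own, without any player trigger.
; Tick feeds a DoOnce that runs a drop, rise cycle spaced by Timer delays, then resets itself.
; Separate timelines rotate the Pivot toward a tilted or zero rotation, lerping from its current rotation each update rather than a stored start value.
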(event `self.ReceiveTick`
  (params (DeltaSeconds :type "Float (single-precision)"))
  (`/Engine/EditorBlueprintResources/StandardMacros.DoOnce` false :!label _label
    (:`Completed`
      (`KismetSystemLibrary.Delay` (`self.timer`))
      (`self.DropPlatform`)
      (`KismetSystemLibrary.Delay` (`self.timer`))
      (`self.Rise Platform`)
      (goto _label :!via `Reset`))))

(event `DropPlatform`
  (bind (_returnvalue_location _returnvalue_rotation _returnvalue_scale) (`KismetMathLibrary.BreakTransform` (`SceneComponent.GetRelativeTransform` (`self.Pivot`))))
  (bind (_direction _open_track) (`Timeline|Drop Platform Timeline` :!via `PlayFromStart`)
    (:`Update`
      (`SceneComponent.K2_SetRelativeTransform` (`self.Pivot`) (`KismetMathLibrary.MakeTransform` _returnvalue_location (`KismetMathLibrary.RLerp` _returnvalue_rotation (struct :`Pitch` -80.0) _open_track) _returnvalue_scale) false false))))

(event `Rise Platform`
  (bind (_returnvalue_location _returnvalue_rotation _returnvalue_scale) (`KismetMathLibrary.BreakTransform` (`SceneComponent.GetRelativeTransform` (`self.Pivot`))))
  (bind (_direction _open_track) (`Timeline|Raise Platform Timeline` :!via `PlayFromStart`)
    (:`Update`
      (`SceneComponent.K2_SetRelativeTransform` (`self.Pivot`) (`KismetMathLibrary.MakeTransform` _returnvalue_location (`KismetMathLibrary.RLerp` _returnvalue_rotation (struct) _open_track) _returnvalue_scale) false false))))

(fn `UserConstructionScript`)