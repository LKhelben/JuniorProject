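; BP_Button is an interactable button that the player toggles on and off with the E key while standing near it.
; Box overlaps with BP_ThirdPersonCharacter enable and disable the actor's input for player controller 0.
; Each E press runs a FlipFlop whose state is written to TIsOn, with no other effect in this graph.
; BeginPlay caches the player character in TPlayer.
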(event `self.ReceiveBeginPlay`
  ;[1 1 1] Sets the value of the player
  (bind _asbp_third_person_character (cast `/Game/ThirdPerson/Blueprints/BP_ThirdPersonCharacter` (`GameplayStatics.GetPlayerCharacter` 0)))
  (set `self.tPlayer` _asbp_third_person_character))

(event `self.Box.OnComponentBeginOverlap`
  (params (OverlappedComponent :type "PrimitiveComponent Object Reference") (OtherActor :type "Actor Object Reference") (OtherComp :type "PrimitiveComponent Object Reference") (OtherBodyIndex :type Integer) (bFromSweep :type Boolean) (SweepResult :type "HitResult Structure (by ref)"))
  ;[1 1 1] Enables/disables input when the player is near
  (cast `/Game/ThirdPerson/Blueprints/BP_ThirdPersonCharacter` OtherActor)
  (`self.EnableInput` (`GameplayStatics.GetPlayerController` 0)))

(event `self.Box.OnComponentEndOverlap`
  (params (OverlappedComponent :type "PrimitiveComponent Object Reference") (OtherActor :type "Actor Object Reference") (OtherComp :type "PrimitiveComponent Object Reference") (OtherBodyIndex :type Integer))
  ;[1 1 1] Enables/disables input when the player is near
  (cast `/Game/ThirdPerson/Blueprints/BP_ThirdPersonCharacter` OtherActor)
  (`self.DisableInput` (`GameplayStatics.GetPlayerController` 0)))

(event `Key|E`
  (params (Key :type "Key Structure"))
  ;[1 1 1] Turns the button on/off wheen pressed
  (:`Pressed`
    (bind _isa (`/Engine/EditorBlueprintResources/StandardMacros.FlipFlop`)
      (:`A`
        _)
      (:`B`
        _))
    (set `self.tIsOn` _isa)))

(fn `UserConstructionScript`)